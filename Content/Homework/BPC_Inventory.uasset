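; BPC_Inventory is an inventory component that holds fixed item slots for medicine, speed boost and coin.
; BeginPlay constructs one item object per type and appends it to ItemSlots.
; AddItem increments a slot's Amount by index.
; UseItem, when Amount is positive, passes the owner to the item's ConsumeMessage and decrements only if it returns true, leaving each effect to the item class.
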(event EventBeginPlay
  (bind _returnvalue (Game|ConstructObjectfromClass self "/Game/Homework/BP_InventoryItem_Medicine.BP_InventoryItem_Medicine_C"))
  (Utilities|Array|Add (Variables|Default|GetItemSlots) _returnvalue)
  (bind _returnvalue_2 (Game|ConstructObjectfromClass self "/Game/Homework/BP_InventoryItem_SpeedBoost.BP_InventoryItem_SpeedBoost_C"))
  (Utilities|Array|Add (Variables|Default|GetItemSlots) _returnvalue_2)
  (bind _returnvalue_3 (Game|ConstructObjectfromClass self "/Game/Homework/BP_InventoryItem_Coin.BP_InventoryItem_Coin_C"))
  (Utilities|Array|Add (Variables|Default|GetItemSlots) _returnvalue_3))

(event EventTick
  (params (DeltaSeconds :type Float%20%28single-precision%29)))

(fn AddItem
  (params (SlotIndex :type Integer))
  (bind _itemslots (Variables|Default|GetItemSlots))
  (bind _output (Utilities|Array|Get(acopy) _itemslots SlotIndex))
  (Variables|/Game/Homework/BP_InventoryItem_Base.BP_InventoryItem_Base_C|SetAmount _output (+ (Variables|/Game/Homework/BP_InventoryItem_Base.BP_InventoryItem_Base_C|GetAmount _output) 1)))

(fn UseItem
  (params (SlotIndex :type Integer))
  (bind _itemslots (Variables|Default|GetItemSlots))
  (bind _output (Utilities|Array|Get(acopy) _itemslots SlotIndex))
  (if (> (Variables|/Game/Homework/BP_InventoryItem_Base.BP_InventoryItem_Base_C|GetAmount _output) 0)
    (bind _bsuccess (Class|BPIConsumeItemable|Consume(Message) _output (Components|GetOwner)))
    (if _bsuccess
      (Variables|/Game/Homework/BP_InventoryItem_Base.BP_InventoryItem_Base_C|SetAmount _output (- (Variables|/Game/Homework/BP_InventoryItem_Base.BP_InventoryItem_Base_C|GetAmount _output) 1)))))